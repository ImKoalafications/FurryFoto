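; BP_FurryFoto_GameMode is the FurryFoto game mode that puts the player on a camera rail when play begins.
; On BeginPlay it casts the player pawn to BP_Player and attaches it to the first CameraRig_Rail found, snapping location and keeping relative rotation and scale.
; It then creates and plays the TestMap_Justin_Sequence level sequence, with a leftover debug "Hello" print along the way.
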(event `self.ReceiveBeginPlay`
  (bind _asbp_player (cast `/Game/FurryFoto/Characters/Blueprints/BP_Player` (`GameplayStatics.GetPlayerPawn` 0)))
  (set `self.Character` _asbp_player)
  (`KismetSystemLibrary.PrintString` "Hello")
  (bind _outactors (`GameplayStatics.GetAllActorsOfClass` "/Script/CinematicCamera.CameraRig_Rail"))
  (`self.K2_AttachToActor` (`self.Character`) (`|GetArrayItem` _outactors) "None" "SnapToTarget" "KeepRelative" "KeepRelative" true)
  (bind (_outactor _returnvalue) (`LevelSequencePlayer.CreateLevelSequencePlayer` "/Game/FurryFoto/Maps/Test/TestMap_Justin_Sequence.TestMap_Justin_Sequence" (make `MovieSceneSequencePlaybackSettings` false)))
  (`MovieSceneSequencePlayer.Play` _returnvalue))

(fn `UserConstructionScript`)